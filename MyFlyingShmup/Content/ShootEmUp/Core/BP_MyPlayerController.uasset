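; Player controller for the ShootEmUp game that tracks the player's score, sets the camera and handles pausing.
; On BeginPlay it switches the view to the level's CameraActor, and on possess it adds the global Enhanced Input mapping context.
; The pause action has the HUD create and show the pause menu, pauses the game and switches to UI-only input with a cursor.
; UnpauseGame restores game-only input.
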(event `AddToPlayerScore`
  (params (`Points To Add` :type "Float (double-precision)"))
  (set `self.PlayerScore` (+ `Points To Add` (`self.PlayerScore`))))

(event `self.ReceiveBeginPlay`
  ; Camera
  (bind _returnvalue (`GameplayStatics.GetActorOfClass` "/Script/Engine.CameraActor"))
  (`self.SetViewTargetWithBlend` _returnvalue))

(event `self.ReceivePossess`
  (params (PossessedPawn :type "Pawn Object Reference"))
  ; Adds Global Inputs
  (bind _asplayer_controller (cast `PlayerController` (`Pawn.GetController` PossessedPawn)))
  (`EnhancedInputSubsystemInterface.AddMappingContext` (pcsubsystem `EnhancedInputLocalPlayerSubsystem` _asplayer_controller) "/Game/ShootEmUp/Inputs/IMC_GlobalInputs.IMC_GlobalInputs" 0 (struct)))

(event `EnhancedInput|/Game/ShootEmUp/Inputs/IA_PauseGame`
  (params (ActionValue :type Boolean) (ElapsedSeconds :type "Float (double-precision)") (TriggeredSeconds :type "Float (double-precision)") (InputAction :type "InputAction Object Reference" :default "/Game/ShootEmUp/Inputs/IA_PauseGame.IA_PauseGame"))
  ; Pause And Unpause
  (:`Triggered`
    (bind _asnew_hud (cast `/Game/ShootEmUp/Core/NewHUD` (`self.GetHUD`)))
    (`/Game/ShootEmUp/Core/NewHUD.CreatePauseMenu` _asnew_hud)
    (bind _pausewidget (`/Game/ShootEmUp/Core/NewHUD.PauseWidget` _asnew_hud))
    (set `Widget.Visibility` "Visible" _pausewidget)
    (`GameplayStatics.SetGamePaused` true)
    (`WidgetBlueprintLibrary.SetInputMode_UIOnlyEx` self _pausewidget)
    (set `self.bShowMouseCursor` true)
    (set `self.Paused` true)))

(event `UnpauseGame`
  ; Pause And Unpause
  (`GameplayStatics.SetGamePaused` false)
  (`WidgetBlueprintLibrary.SetInputMode_GameOnly` self)
  (set `self.bShowMouseCursor` false)
  (set `self.Paused` false))

(fn `UserConstructionScript`)