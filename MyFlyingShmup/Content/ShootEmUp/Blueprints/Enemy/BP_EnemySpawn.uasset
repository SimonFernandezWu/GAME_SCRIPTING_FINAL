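; Enemy spawner for a shoot 'em up that continuously sends random enemy types along level paths.
; On BeginPlay it caches all BP_EnemyPath actors and starts a fast looping timer, spawning at a random spline's first point in local space.
; Each BP_BaseEnemy gets a separately randomized path, starts moving, then fires after a short delay.
; A failed cast destroys the spawner itself.
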(event `self.ReceiveBeginPlay`
  (`self.GetAllPaths`)
  (`self.StartTimer`))

(event `GetAllPaths`
  (bind _outactors (`GameplayStatics.GetAllActorsOfClass` "/Game/ShootEmUp/Blueprints/Enemy/BP_EnemyPath.BP_EnemyPath_C"))
  (set `self.PawnPaths` _outactors))

(event `StartTimer`
  (`KismetSystemLibrary.K2_SetTimerDelegate` (delegate `SpawnEnemy`) 0.5 true))

(event `SpawnEnemy`
  (bind _outitem (`KismetArrayLibrary.Array_Random` (`self.PawnPaths`)))
  ; Spawning on path
  (bind _output_get (set `self.NewVar` (`SplineComponent.GetTransformAtSplinePoint` (`/Game/ShootEmUp/Blueprints/Enemy/BP_EnemyPath.Spline` _outitem) 0 "Local" false)))
  (bind _returnvalue (`|SpawnActorFromClass` (`KismetArrayLibrary.Array_Random` (`self.AllEnemies`)) (`KismetMathLibrary.MakeTransform` (.location _output_get) (.rotation _output_get)) "Undefined" "MultiplyWithRoot" null null))
  (bind _asbp_base_enemy (cast `/Game/ShootEmUp/Blueprints/Enemy/BP_BaseEnemy` _returnvalue)
    (:`then`
      (set `/Game/ShootEmUp/Blueprints/Enemy/BP_BaseEnemy.Path` _outitem _asbp_base_enemy)
      (`/Game/ShootEmUp/Blueprints/Enemy/BP_BaseEnemy.StartMovingAlongPath` _asbp_base_enemy)
      (`KismetSystemLibrary.Delay` 0.1)
      (`/Game/ShootEmUp/Blueprints/Enemy/BP_BaseEnemy.BeginFire` _asbp_base_enemy))
    (:`CastFailed`
      (`self.K2_DestroyActor`))))

(fn `UserConstructionScript`)