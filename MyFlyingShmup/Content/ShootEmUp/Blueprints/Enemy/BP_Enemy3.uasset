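; BP_Enemy3 is a shoot 'em up enemy variant that extends a parent class, setting its own Speed on BeginPlay.
; On overlap it subtracts the other actor's AC_Properties Damage from its own Health, after running the parent's overlap logic.
; When Health reaches zero or below, it spawns a scaled-up Niagara effect at its location and destroys itself, with short delays before each step.
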(event `self.ReceiveBeginPlay`
  (`parent.ReceiveBeginPlay`)
  (set `self.Speed` 0.3))

(event `self.ReceiveActorBeginOverlap`
  (params (OtherActor :type "Actor Object Reference"))
  (bind _ac_properties (`self.AC_Properties`))
  ; Health
  (`parent.ReceiveActorBeginOverlap` null)
  (bind _output_get (set `/Game/ShootEmUp/Blueprints/AC_Properties.Health` (- (`/Game/ShootEmUp/Blueprints/AC_Properties.Health` _ac_properties) (`/Game/ShootEmUp/Blueprints/AC_Properties.Damage` (`self.GetComponentByClass` OtherActor "/Game/ShootEmUp/Blueprints/AC_Properties.AC_Properties_C"))) _ac_properties))
  (if (<= _output_get 0.0)
    (`KismetSystemLibrary.Delay` 0.2)
    (`NiagaraFunctionLibrary.SpawnSystemAtLocation` "/Game/ShootEmUp/Basic_VFX/Niagara/NS_Basic_2.NS_Basic_2" (`self.K2_GetActorLocation`) (struct) (3.0 3.0 3.0))
    (`KismetSystemLibrary.Delay` 0.1)
    (`self.K2_DestroyActor`)))

(fn `UserConstructionScript`
  (`parent.UserConstructionScript`))