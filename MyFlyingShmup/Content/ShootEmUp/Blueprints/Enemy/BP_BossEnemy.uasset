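; Shoot-em-up boss dropship that glides in on BeginPlay and ends the game with a win screen when defeated.
; A looping timer fires missiles alternately from two points, each homing on the player briefly.
; Overlaps damage two engines and a core via AC_Properties, flashing them; destroying the core pauses missiles.
; Tick polls the three death flags without a one-shot guard, spawning explosions and, after a delay, the win widget.
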(event `self.ReceiveBeginPlay`
  (`KismetSystemLibrary.MoveComponentTo` (`self.DefaultSceneRoot`) (3500.0 0.0 70.0) (struct) true false 3.0)
  (bind _returnvalue (`KismetSystemLibrary.K2_SetTimerDelegate` (delegate `Missile`) 5.0 true))
  (set `self.Handle` _returnvalue))

(event `Missile`
  (bind _returnvalue (`self.GetComponentByClass` (`GameplayStatics.GetPlayerPawn` 0) "/Script/Engine.SphereComponent"))
  (`/Engine/EditorBlueprintResources/StandardMacros.FlipFlop`
    (:`A`
      (bind _returnvalue_2 (`|SpawnActorFromClass` "/Game/ShootEmUp/Blueprints/Enemy/BPC_BossMissile.BPC_BossMissile_C" (`KismetMathLibrary.MakeTransform` (`SceneComponent.K2_GetComponentLocation` (`self.FireLocation1`)) (struct :`Yaw` -180.0)) "Undefined" "MultiplyWithRoot" null 0.0 null))
      (bind _projectilemovement (`/Game/ShootEmUp/Blueprints/Enemy/BPC_BossMissile.ProjectileMovement` _returnvalue_2))
      (set `ProjectileMovementComponent.bIsHomingProjectile` true _projectilemovement)
      (set `ProjectileMovementComponent.HomingTargetComponent` _returnvalue _projectilemovement)
      (`KismetSystemLibrary.Delay` 5.0)
      (set `ProjectileMovementComponent.bIsHomingProjectile` false _projectilemovement))
    (:`B`
      (bind _returnvalue_3 (`|SpawnActorFromClass` "/Game/ShootEmUp/Blueprints/Enemy/BPC_BossMissile.BPC_BossMissile_C" (`KismetMathLibrary.MakeTransform` (`SceneComponent.K2_GetComponentLocation` (`self.FireLocation2`)) (struct :`Yaw` -180.0)) "Undefined" "MultiplyWithRoot" null 0.0 null))
      (bind _projectilemovement_2 (`/Game/ShootEmUp/Blueprints/Enemy/BPC_BossMissile.ProjectileMovement` _returnvalue_3))
      (set `ProjectileMovementComponent.bIsHomingProjectile` true _projectilemovement_2)
      (set `ProjectileMovementComponent.HomingTargetComponent` _returnvalue _projectilemovement_2)
      (`KismetSystemLibrary.Delay` 5.0)
      (set `ProjectileMovementComponent.bIsHomingProjectile` false _projectilemovement_2))))

(event `self.ReceiveTick`
  (params (DeltaSeconds :type "Float (single-precision)"))
  (bind _returnvalue (`GameplayStatics.GetPlayerController` 0))
  (if (`self.Dead1`)
    (if (`self.Dead2`)
      (if (`self.Dead3`)
        (`NiagaraFunctionLibrary.SpawnSystemAtLocation` "/Game/ShootEmUp/Basic_VFX/Niagara/NS_Basic_13.NS_Basic_13" (`SceneComponent.K2_GetComponentLocation` (`self.Dropship_R35_Engine1`)) (struct) (5.0 5.0 5.0))
        (`KismetSystemLibrary.Delay` 10.0)
        (bind _returnvalue_2 (`|CreateWidget` "/Game/ShootEmUp/UI/BP_WinScreen.BP_WinScreen_C" _returnvalue))
        (bind _output_get (set `self.NewVar` _returnvalue_2))
        (`UserWidget.AddToViewport` _output_get 0)
        (`WidgetBlueprintLibrary.SetInputMode_UIOnlyEx` _returnvalue _returnvalue_2)))))

(event `self.Box1.OnComponentBeginOverlap`
  (params (OverlappedComponent :type "PrimitiveComponent Object Reference") (OtherActor :type "Actor Object Reference") (OtherComp :type "PrimitiveComponent Object Reference") (OtherBodyIndex :type Integer) (bFromSweep :type Boolean) (SweepResult :type "HitResult Structure (by ref)"))
  (bind _dropship_r35_engine1 (`self.Dropship_R35_Engine1`))
  ; Engine 1 HP
  (if (<= (`self.Health Engine 1`) 0.0)
    (`NiagaraFunctionLibrary.SpawnSystemAtLocation` "/Game/ShootEmUp/Basic_VFX/Niagara/NS_Basic_6.NS_Basic_6" (`SceneComponent.K2_GetComponentLocation` (`self.Dropship_R35_Engine1`)) (struct) (5.0 5.0 5.0))
    (`MeshComponent.SetOverlayMaterial` (`self.Dropship_R35_Engine1`) "/Game/ShootEmUp/Materials/MI_FlashingEnemyMaterial.MI_FlashingEnemyMaterial")
    (`ActorComponent.K2_DestroyComponent` (`self.Box1`))
    (set `self.Dead1` true)
    (else
      (set `self.Health Engine 1` (`KismetMathLibrary.FClamp` (- (`self.Health Engine 1`) (`/Game/ShootEmUp/Blueprints/AC_Properties.Damage` (`self.GetComponentByClass` OtherActor "/Game/ShootEmUp/Blueprints/AC_Properties.AC_Properties_C"))) 0.0 1000.0))
      (`MeshComponent.SetOverlayMaterial` _dropship_r35_engine1 "/Game/ShootEmUp/Materials/MI_FlashingEnemyMaterial.MI_FlashingEnemyMaterial")
      (`KismetSystemLibrary.Delay` 0.2)
      (`MeshComponent.SetOverlayMaterial` _dropship_r35_engine1 null)
      (`AudioComponent.Play` (`self.SciFi_Shot_P2__22_`) 0.0))))

(event `self.Capsule.OnComponentBeginOverlap`
  (params (OverlappedComponent :type "PrimitiveComponent Object Reference") (OtherActor :type "Actor Object Reference") (OtherComp :type "PrimitiveComponent Object Reference") (OtherBodyIndex :type Integer) (bFromSweep :type Boolean) (SweepResult :type "HitResult Structure (by ref)"))
  (bind _dropship_r351 (`self.Dropship_R351`))
  ; Core HP
  (if (<= (`self.Health Core`) 0.0)
    (`NiagaraFunctionLibrary.SpawnSystemAtLocation` "/Game/ShootEmUp/Basic_VFX/Niagara/NS_Basic_6.NS_Basic_6" (`SceneComponent.K2_GetComponentLocation` (`self.Dropship_R351`)) (struct) (5.0 5.0 5.0))
    (`MeshComponent.SetOverlayMaterial` (`self.Dropship_R351`) "/Game/ShootEmUp/Materials/MI_FlashingEnemyMaterial.MI_FlashingEnemyMaterial")
    (`ActorComponent.K2_DestroyComponent` (`self.Capsule`))
    (`KismetSystemLibrary.K2_PauseTimerHandle` (`self.Handle`))
    (set `self.Dead2` true)
    (else
      (set `self.Health Core` (`KismetMathLibrary.FClamp` (- (`self.Health Core`) (`/Game/ShootEmUp/Blueprints/AC_Properties.Damage` (`self.GetComponentByClass` OtherActor "/Game/ShootEmUp/Blueprints/AC_Properties.AC_Properties_C"))) 0.0 1000.0))
      (`MeshComponent.SetOverlayMaterial` _dropship_r351 "/Game/ShootEmUp/Materials/MI_FlashingEnemyMaterial.MI_FlashingEnemyMaterial")
      (`KismetSystemLibrary.Delay` 0.2)
      (`MeshComponent.SetOverlayMaterial` _dropship_r351 null)
      (`AudioComponent.Play` (`self.SciFi_Shot_P2__22_`) 0.0))))

(event `self.Box.OnComponentBeginOverlap`
  (params (OverlappedComponent :type "PrimitiveComponent Object Reference") (OtherActor :type "Actor Object Reference") (OtherComp :type "PrimitiveComponent Object Reference") (OtherBodyIndex :type Integer) (bFromSweep :type Boolean) (SweepResult :type "HitResult Structure (by ref)"))
  (bind _dropship_r35_engine2 (`self.Dropship_R35_Engine2`))
  ; Engine 2 HP
  (if (<= (`self.Health Engine 2`) 0.0)
    (`NiagaraFunctionLibrary.SpawnSystemAtLocation` "/Game/ShootEmUp/Basic_VFX/Niagara/NS_Basic_6.NS_Basic_6" (`SceneComponent.K2_GetComponentLocation` (`self.Dropship_R35_Engine2`)) (struct) (5.0 5.0 5.0))
    (`MeshComponent.SetOverlayMaterial` (`self.Dropship_R35_Engine2`) "/Game/ShootEmUp/Materials/MI_FlashingEnemyMaterial.MI_FlashingEnemyMaterial")
    (`ActorComponent.K2_DestroyComponent` (`self.Box`))
    (set `self.Dead3` true)
    (else
      (set `self.Health Engine 2` (`KismetMathLibrary.FClamp` (- (`self.Health Engine 2`) (`/Game/ShootEmUp/Blueprints/AC_Properties.Damage` (`self.GetComponentByClass` OtherActor "/Game/ShootEmUp/Blueprints/AC_Properties.AC_Properties_C"))) 0.0 1000.0))
      (`MeshComponent.SetOverlayMaterial` _dropship_r35_engine2 "/Game/ShootEmUp/Materials/MI_FlashingEnemyMaterial.MI_FlashingEnemyMaterial")
      (`KismetSystemLibrary.Delay` 0.2)
      (`MeshComponent.SetOverlayMaterial` _dropship_r35_engine2 null)
      (`AudioComponent.Play` (`self.SciFi_Shot_P2__22_`) 0.0))))

(fn `UserConstructionScript`)