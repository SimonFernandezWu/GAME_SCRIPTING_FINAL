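; Base enemy for a shoot 'em up that follows a spline path, fires at the player and rewards score and pickups.
; A timeline moves it at constant velocity along the spline, then destroys it.
; A delay loop spawns bullets yawed toward the player, using AC_Properties damage, while overlaps flash meshes and play sound.
; Any destruction, including reaching path end, awards health-based points and independently rolls three pickup drops.
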(event `self.ReceiveBeginPlay`
  (bind _ac_properties (`self.AC_Properties`))
  (bind _health (`/Game/ShootEmUp/Blueprints/AC_Properties.Health` _ac_properties))
  (set `self.Health` _health)
  (set `/Game/ShootEmUp/Blueprints/AC_Properties.Points` (`KismetMathLibrary.FTrunc` _health) _ac_properties))

(event `StartMovingAlongPath`
  (bind _spline (`/Game/ShootEmUp/Blueprints/Enemy/BP_EnemyPath.Spline` (`self.Path`)))
  ; Moving across path
  (`/Engine/EditorBlueprintResources/StandardMacros.DoOnce` false
    (:`Completed`
      (bind (_direction _time) (`Timeline|Timeline`)
        (:`Update`
          (`TimelineComponent.SetPlayRate` (`self.Timeline`) (`self.Speed`))
          (`self.K2_SetActorTransform` (`KismetMathLibrary.MakeTransform` (`SplineComponent.GetLocationAtTime` _spline _time "World" true) (`SplineComponent.GetRotationAtTime` _spline _time "World" true))))
        (:`Finished`
          (`self.K2_DestroyActor`))))))

(event `BeginFire`
  (params (`Fire Interval` :type "Float (double-precision)") (`Bullet Class` :type "Actor Class Reference"))
  (bind _returnvalue_location (`KismetMathLibrary.BreakTransform` (`self.GetTransform`)))
  (bind _returnvalue (`self.GetComponentByClass` "/Game/ShootEmUp/Blueprints/AC_Properties.AC_Properties_C"))
  ; SpawnBullets
  (if (`KismetSystemLibrary.IsValid` _returnvalue)
    (bind _returnvalue_2 (`GameplayStatics.GetActorOfClass` "/Game/ShootEmUp/Blueprints/Player/BP_PlayerPawn.BP_PlayerPawn_C"))
    (bind _returnvalue_location_2 (`KismetMathLibrary.BreakTransform` (`self.GetTransform` _returnvalue_2)))
    (bind (_returnvalue_roll _returnvalue_pitch _returnvalue_yaw) (`KismetMathLibrary.BreakRotator` (`KismetMathLibrary.FindLookAtRotation` _returnvalue_location _returnvalue_location_2)))
    (`|SpawnActorFromClass` `Bullet Class` (`KismetMathLibrary.MakeTransform` _returnvalue_location (`KismetMathLibrary.MakeRotator` 0.0 0.0 _returnvalue_yaw)) "Undefined" "MultiplyWithRoot" null (`/Game/ShootEmUp/Blueprints/AC_Properties.Damage` _returnvalue) null :!label _label)
    (`KismetSystemLibrary.Delay` `Fire Interval`)
    (goto _label)))

(event `self.ReceiveActorBeginOverlap`
  (params (OtherActor :type "Actor Object Reference"))
  ; Hit overlay and sound
  (for _array_element (`self.K2_GetComponentsByClass` "/Script/Engine.StaticMeshComponent")
    (`MeshComponent.SetOverlayMaterial` _array_element "/Game/ShootEmUp/Materials/MI_FlashingEnemyMaterial.MI_FlashingEnemyMaterial")
    (`KismetSystemLibrary.Delay` 0.2)
    (`MeshComponent.SetOverlayMaterial` _array_element null))
  (`AudioComponent.Play` (`self.SciFi_Shot_P2__90_`) 0.0))

(event `self.ReceiveEndPlay`
  (params (EndPlayReason :type "EEndPlayReason Enum" :default "Destroyed"))
  (bind _returnvalue_location (`KismetMathLibrary.BreakTransform` (`self.GetTransform`)))
  (bind _returnvalue_location_2 (`KismetMathLibrary.BreakTransform` (`self.GetTransform`)))
  (bind _returnvalue_location_3 (`KismetMathLibrary.BreakTransform` (`self.GetTransform`)))
  (switch `EEndPlayReason` EndPlayReason
    (:`Destroyed`
      ; Add to player score
      (bind _asbp_my_player_controller (cast `/Game/ShootEmUp/Core/BP_MyPlayerController` (`GameplayStatics.GetPlayerController` 0)))
      (`/Game/ShootEmUp/Core/BP_MyPlayerController.AddToPlayerScore` _asbp_my_player_controller (`KismetMathLibrary.Conv_IntToDouble` (`/Game/ShootEmUp/Blueprints/AC_Properties.Points` (`self.AC_Properties`))))
      ; Spawns Pickups
      (`|ExecutionSequence`
        (:`then_0`
          (if (< (`KismetMathLibrary.RandomFloat`) 0.2)
            (`|SpawnActorFromClass` "/Game/ShootEmUp/Blueprints/PickUps/BP_Circuit.BP_Circuit_C" (`KismetMathLibrary.MakeTransform` _returnvalue_location_3 (struct :`Yaw` 180.0)) "Undefined" "MultiplyWithRoot" null (struct :`R` 0.026234 :`G` 1.0 :`A` 1.0) null)))
        (:`then_1`
          (if (< (`KismetMathLibrary.RandomFloat`) 0.1)
            (`|SpawnActorFromClass` "/Game/ShootEmUp/Blueprints/PickUps/BP_HealthPickup.BP_HealthPickup_C" (`KismetMathLibrary.MakeTransform` _returnvalue_location_2 (struct :`Yaw` 180.0)) "Undefined" "MultiplyWithRoot" null (struct :`R` 1.0) null)))
        (:`then_2`
          (if (< (`KismetMathLibrary.RandomFloat`) 0.05)
            (`|SpawnActorFromClass` "/Game/ShootEmUp/Blueprints/PickUps/BP_PickUp_ShootingMode.BP_PickUp_ShootingMode_C" (`KismetMathLibrary.MakeTransform` _returnvalue_location (struct :`Yaw` 180.0)) "Undefined" "MultiplyWithRoot" null (struct :`R` 1.0 :`B` 0.830507 :`A` 1.0) null)))))))

(fn `UserConstructionScript`)