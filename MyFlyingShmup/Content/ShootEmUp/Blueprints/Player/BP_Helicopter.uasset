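; BP_Helicopter is the player-controlled helicopter pawn for the shoot-em-up.
; On possession it adds the Enhanced Input movement mapping, and four directional actions feed world-axis vectors into FloatingPawnMovement.
; Tick banks the body through actor pitch, interpolating toward a target chosen from left/right input and leveling when both or neither are held.
; Two RotatingMovement components, bound to the propellers at BeginPlay, spin them, replacing an unused manual rotation method.
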(event `self.ReceivePossessed`
  (params (NewController :type "Controller Object Reference"))
  ; Movement_KeyBinds
  (bind _asplayer_controller (cast `PlayerController` NewController))
  (`EnhancedInputSubsystemInterface.AddMappingContext` (pcsubsystem `EnhancedInputLocalPlayerSubsystem` _asplayer_controller) "/Game/ShootEmUp/Inputs/IMC_PlayerMovement.IMC_PlayerMovement" 0 (struct)))

(event `EnhancedInput|/Game/ShootEmUp/Inputs/IA_MoveRight`
  (params (ActionValue :type Boolean) (ElapsedSeconds :type "Float (double-precision)") (TriggeredSeconds :type "Float (double-precision)") (InputAction :type "InputAction Object Reference" :default "/Game/ShootEmUp/Inputs/IA_MoveRight.IA_MoveRight"))
  ; Movement_KeyBinds
  (:`Triggered`
    (`PawnMovementComponent.AddInputVector` (`self.FloatingPawnMovement`) (1.0 0.0 0.0) false)))

(event `EnhancedInput|/Game/ShootEmUp/Inputs/IA_MoveLeft`
  (params (ActionValue :type Boolean) (ElapsedSeconds :type "Float (double-precision)") (TriggeredSeconds :type "Float (double-precision)") (InputAction :type "InputAction Object Reference" :default "/Game/ShootEmUp/Inputs/IA_MoveLeft.IA_MoveLeft"))
  ; Movement_KeyBinds
  (:`Triggered`
    (`PawnMovementComponent.AddInputVector` (`self.FloatingPawnMovement`) (-1.0 0.0 0.0) false)))

(event `EnhancedInput|/Game/ShootEmUp/Inputs/IA_MoveBackwards`
  (params (ActionValue :type Boolean) (ElapsedSeconds :type "Float (double-precision)") (TriggeredSeconds :type "Float (double-precision)") (InputAction :type "InputAction Object Reference" :default "/Game/ShootEmUp/Inputs/IA_MoveBackwards.IA_MoveBackwards"))
  ; Movement_KeyBinds
  (:`Triggered`
    (`PawnMovementComponent.AddInputVector` (`self.FloatingPawnMovement`) (0.0 1.0 0.0) false)))

(event `EnhancedInput|/Game/ShootEmUp/Inputs/IA_MoveFowards`
  (params (ActionValue :type Boolean) (ElapsedSeconds :type "Float (double-precision)") (TriggeredSeconds :type "Float (double-precision)") (InputAction :type "InputAction Object Reference" :default "/Game/ShootEmUp/Inputs/IA_MoveFowards.IA_MoveFowards"))
  ; Movement_KeyBinds
  (:`Triggered`
    (`PawnMovementComponent.AddInputVector` (`self.FloatingPawnMovement`) (0.0 -1.0 0.0) false)))

(event `self.ReceiveBeginPlay`
  ; Propeller Movement Method 2 (Better)
  (`MovementComponent.SetUpdatedComponent` (`self.RotatingMovement`) (`self.BPropeller`))
  (`MovementComponent.SetUpdatedComponent` (`self.RotatingMovement1`) (`self.FPropeller`)))

(event `self.ReceiveTick`
  (params (DeltaSeconds :type "Float (single-precision)"))
  (bind _returnvalue (`|GetInputActionValue`))
  (bind _returnvalue_2 (`|GetInputActionValue`))
  (`|ExecutionSequence`
    (:`then_0`
      (set `self.Delta Seconds` DeltaSeconds)
      (bind _output_get (set `self.Current Rotation` (`KismetMathLibrary.FInterpTo` (`self.Current Rotation`) (`self.Target Rotation`) (`self.Delta Seconds`) 1.0)))
      (`self.K2_SetActorRotation` (`KismetMathLibrary.MakeRotator` 0.0 (* _output_get 30.0)))
      (set `self.Target Rotation` (`KismetMathLibrary.SelectFloat` 0.0 (`KismetMathLibrary.SelectFloat` 1.0 -1.0 (`|GetInputActionValue`)) (or (and _returnvalue_2 _returnvalue) (`KismetMathLibrary.BooleanNOR` _returnvalue_2 _returnvalue)))))))

(fn `UserConstructionScript`)