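; BP_MouseShooterPawn is a mouse-controlled shooter pawn for the ShootEmUp game.
; On possession it adds the mouse mapping context and shows a crosshair cursor.
; Move input traces under the cursor, turns the pawn toward the hit point and drives FloatingPawnMovement forward, using the 2D distance as max speed so it eases in.
; Shoot input spawns BP_Bullet at the Arrow, rate-limited by a DoOnce and Delay.
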(event `EnhancedInput|/Game/ShootEmUp/Inputs/IA_MoveWithMouse`
  (params (ActionValue :type Boolean) (ElapsedSeconds :type "Float (double-precision)") (TriggeredSeconds :type "Float (double-precision)") (InputAction :type "InputAction Object Reference" :default "/Game/ShootEmUp/Inputs/IA_MoveWithMouse.IA_MoveWithMouse"))
  (bind _returnvalue (* (`self.K2_GetActorLocation`) (1.0 1.0 0.0)))
  ; Move With Mouse
  (:`Triggered`
    (bind _returnvalue_2 (`WidgetLayoutLibrary.GetMousePositionOnViewport`))
    (bind (_worldposition _worlddirection) (`GameplayStatics.DeprojectScreenToWorld` (`self.As Player Controller`) (* _returnvalue_2 (`WidgetLayoutLibrary.GetViewportScale`))))
    (bind _outhit (`KismetSystemLibrary.LineTraceSingle` _worldposition (+ _worldposition (* _worlddirection 5000.0)) "TraceTypeQuery1"))
    (bind _returnvalue_3 (* (`.Location` (`GameplayStatics.BreakHitResult` _outhit)) (1.0 1.0 0.0)))
    (`self.K2_SetActorRotation` (`KismetMathLibrary.FindLookAtRotation` _returnvalue _returnvalue_3))
    (`PawnMovementComponent.AddInputVector` (`self.FloatingPawnMovement`) (`self.GetActorForwardVector`) false)
    (set `FloatingPawnMovement.MaxSpeed` (`KismetMathLibrary.Distance2D` (`KismetMathLibrary.Conv_VectorToVector2D` _returnvalue) (`KismetMathLibrary.Conv_VectorToVector2D` _returnvalue_3)) (`self.FloatingPawnMovement`))))

(event `self.ReceiveTick`
  (params (DeltaSeconds :type "Float (single-precision)"))
  ; Move With Mouse
)

(event `self.ReceivePossessed`
  (params (NewController :type "Controller Object Reference"))
  (bind _as_player_controller (`self.As Player Controller`))
  ; Cast IMC
  (bind _asplayer_controller (cast `PlayerController` NewController))
  (set `self.As Player Controller` _asplayer_controller)
  (`EnhancedInputSubsystemInterface.AddMappingContext` (pcsubsystem `EnhancedInputLocalPlayerSubsystem` _asplayer_controller) "/Game/ShootEmUp/Inputs/IMC_MouseControls.IMC_MouseControls" 0 (struct))
  (set `PlayerController.bShowMouseCursor` true _as_player_controller)
  (set `PlayerController.CurrentMouseCursor` "Crosshairs" _as_player_controller))

(event `EnhancedInput|/Game/ShootEmUp/Inputs/IA_ShootWithMouse`
  (params (ActionValue :type "Vector2D Structure") (ElapsedSeconds :type "Float (double-precision)") (TriggeredSeconds :type "Float (double-precision)") (InputAction :type "InputAction Object Reference" :default "/Game/ShootEmUp/Inputs/IA_ShootWithMouse.IA_ShootWithMouse"))
  (bind _arrow (`self.Arrow`))
  (:`Triggered`
    ; Single
    (`/Engine/EditorBlueprintResources/StandardMacros.DoOnce` false :!label _label
      (:`Completed`
        (`|SpawnActorFromClass` "/Game/ShootEmUp/Blueprints/Player/BP_Bullet.BP_Bullet_C" (`KismetMathLibrary.MakeTransform` (`SceneComponent.K2_GetComponentLocation` _arrow) (`SceneComponent.K2_GetComponentRotation` _arrow)) "Undefined" "MultiplyWithRoot" null null)
        (`KismetSystemLibrary.Delay` 0.15)
        (goto _label :!via `Reset`)))))

(fn `UserConstructionScript`)