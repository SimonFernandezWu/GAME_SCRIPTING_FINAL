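; Player ship pawn for a shoot 'em up, with Enhanced Input movement and banking tilt.
; Primary fire shoots twin bullets and alternating-side missiles, or a bullet fan during Frenzy; secondary fire cycles a shooting mode that firing ignores.
; Overlaps read actor components for damage or pickups (health, fire rate, money, Frenzy), updating HUD and GameInstance.
; Death removes a HUD life icon, then respawns at PlayerStart or shows game over; upgrade logic is unfinished.
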(event `self.ReceivePossessed`
  (params (NewController :type "Controller Object Reference"))
  ; Cast
  (bind _asplayer_controller (cast `PlayerController` NewController))
  (`EnhancedInputSubsystemInterface.AddMappingContext` (pcsubsystem `EnhancedInputLocalPlayerSubsystem` _asplayer_controller) "/Game/ShootEmUp/Inputs/IMC_PlayerMovement.IMC_PlayerMovement" 0 (struct))
  (`self.InitializeHealth`))

(event `EnhancedInput|/Game/ShootEmUp/Inputs/IA_PrimaryFire`
  (params (ActionValue :type Boolean) (ElapsedSeconds :type "Float (double-precision)") (TriggeredSeconds :type "Float (double-precision)") (InputAction :type "InputAction Object Reference" :default "/Game/ShootEmUp/Inputs/IA_PrimaryFire.IA_PrimaryFire"))
  (bind _returnvalue (`SceneComponent.K2_GetComponentLocation` (`self.Primary Fire Location`)))
  ; Shooting
  (:`Triggered`
    (`|ExecutionSequence`
      (:`then_0`
        ; Double
        (if (not (`self.FrenzyPowerup`))
          (`/Engine/EditorBlueprintResources/StandardMacros.DoOnce` false :!label _label
            (:`Completed`
              (`|SpawnActorFromClass` "/Game/ShootEmUp/Blueprints/Player/BP_Bullet.BP_Bullet_C" (`KismetMathLibrary.MakeTransform` (+ _returnvalue (0.0 150.0 0.0))) "Undefined" "MultiplyWithRoot" null null)
              (`|SpawnActorFromClass` "/Game/ShootEmUp/Blueprints/Player/BP_Bullet.BP_Bullet_C" (`KismetMathLibrary.MakeTransform` (+ _returnvalue (0.0 -150.0 0.0))) "Undefined" "MultiplyWithRoot" null null)
              (`KismetSystemLibrary.Delay` (`/Game/ShootEmUp/Blueprints/AC_Properties.Firerate` (`self.AC_Properties`)))
              (goto _label :!via `Reset`)))))
      (:`then_1`
        ; Missile
        (if (not (`self.FrenzyPowerup`))
          (`/Engine/EditorBlueprintResources/StandardMacros.DoOnce` false :!label _label_2
            (:`Completed`
              (bind _returnvalue_2 (`|SpawnActorFromClass` "/Game/ShootEmUp/Blueprints/Player/BP_Missile.BP_Missile_C" (`KismetMathLibrary.MakeTransform` (`SceneComponent.K2_GetComponentLocation` (`self.Primary Fire Location`))) "Undefined" "MultiplyWithRoot" null null))
              (`/Engine/EditorBlueprintResources/StandardMacros.FlipFlop`
                (:`A`
                  (set `/Game/ShootEmUp/Blueprints/Player/BP_Missile.RightSide` true _returnvalue_2)
                  (`KismetSystemLibrary.Delay` 1.0)
                  (goto _label_2 :!via `Reset`))
                (:`B`
                  (set `/Game/ShootEmUp/Blueprints/Player/BP_Missile.RightSide` false _returnvalue_2)
                  (`KismetSystemLibrary.Delay` 1.0)
                  (goto _label_2 :!via `Reset`)))))))
      (:`then_2`
        (if (`self.FrenzyPowerup`)
          ; Frenzy PU
          (`/Engine/EditorBlueprintResources/StandardMacros.DoOnce` false :!label _label_3
            (:`Completed`
              (for _index (range 1 (+ (`self.NumBullets`) 1))
                (`|SpawnActorFromClass` "/Game/ShootEmUp/Blueprints/Player/BP_Bullet.BP_Bullet_C" (`KismetMathLibrary.MakeTransform` (`SceneComponent.K2_GetComponentLocation` (`self.Primary Fire Location`)) (`KismetMathLibrary.MakeRotator` 0.0 0.0 (- (* _index 10.0) (* (`self.NumBullets`) 5.0) 5.0))) "Undefined" "MultiplyWithRoot" null null)
                (`KismetSystemLibrary.Delay` 0.6)
                (goto _label_3 :!via `Reset`)))))))))

(event `EnhancedInput|/Game/ShootEmUp/Inputs/IA_MoveFowards`
  (params (ActionValue :type Boolean) (ElapsedSeconds :type "Float (double-precision)") (TriggeredSeconds :type "Float (double-precision)") (InputAction :type "InputAction Object Reference" :default "/Game/ShootEmUp/Inputs/IA_MoveFowards.IA_MoveFowards"))
  ; Base Controls
  (:`Triggered`
    (`PawnMovementComponent.AddInputVector` (`self.FloatingPawnMovement`) (1.0 0.0 0.0) false)))

(event `EnhancedInput|/Game/ShootEmUp/Inputs/IA_MoveBackwards`
  (params (ActionValue :type Boolean) (ElapsedSeconds :type "Float (double-precision)") (TriggeredSeconds :type "Float (double-precision)") (InputAction :type "InputAction Object Reference" :default "/Game/ShootEmUp/Inputs/IA_MoveBackwards.IA_MoveBackwards"))
  ; Base Controls
  (:`Triggered`
    (`PawnMovementComponent.AddInputVector` (`self.FloatingPawnMovement`) (-1.0 0.0 0.0) false)))

(event `SwitchShootingModes`
  ; ModeSwitch
  (bind _output_get (set `self.ShootingMode` (mod (+ (`self.ShootingMode`) 1) (+ (`self.MaxShootingMode`) 1))))
  (`KismetSystemLibrary.PrintString` (`KismetStringLibrary.Conv_IntToString` _output_get)))

(event `EnhancedInput|/Game/ShootEmUp/Inputs/IA_MoveRight`
  (params (ActionValue :type Boolean) (ElapsedSeconds :type "Float (double-precision)") (TriggeredSeconds :type "Float (double-precision)") (InputAction :type "InputAction Object Reference" :default "/Game/ShootEmUp/Inputs/IA_MoveRight.IA_MoveRight"))
  ; Base Controls
  (:`Triggered`
    (`PawnMovementComponent.AddInputVector` (`self.FloatingPawnMovement`) (0.0 1.0 0.0) false)))

(event `EnhancedInput|/Game/ShootEmUp/Inputs/IA_MoveLeft`
  (params (ActionValue :type Boolean) (ElapsedSeconds :type "Float (double-precision)") (TriggeredSeconds :type "Float (double-precision)") (InputAction :type "InputAction Object Reference" :default "/Game/ShootEmUp/Inputs/IA_MoveLeft.IA_MoveLeft"))
  ; Base Controls
  (:`Triggered`
    (`PawnMovementComponent.AddInputVector` (`self.FloatingPawnMovement`) (0.0 -1.0 0.0) false)))

(event `EnhancedInput|/Game/ShootEmUp/Inputs/IA_SecondaryFire`
  (params (ActionValue :type Boolean) (ElapsedSeconds :type "Float (double-precision)") (TriggeredSeconds :type "Float (double-precision)") (InputAction :type "InputAction Object Reference" :default "/Game/ShootEmUp/Inputs/IA_SecondaryFire.IA_SecondaryFire"))
  ; ModeSwitch
  (:`Triggered`
    (`/Engine/EditorBlueprintResources/StandardMacros.DoOnce` false :!label _label_4
      (:`Completed`
        (`self.SwitchShootingModes`)
        (`KismetSystemLibrary.Delay` 0.5)
        (goto _label_4 :!via `Reset`)))))

(event `self.ReceiveTick`
  (params (DeltaSeconds :type "Float (single-precision)"))
  (bind _returnvalue (`|GetInputActionValue`))
  (bind _returnvalue_2 (`|GetInputActionValue`))
  ; Movement Tilt
  (set `self.Delta Seconds` DeltaSeconds)
  (bind _output_get (set `self.Current` (`KismetMathLibrary.FInterpTo` (`self.Current`) (`self.Target`) (`self.Delta Seconds`) 1.0)))
  (`self.K2_SetActorRotation` (`KismetMathLibrary.MakeRotator` (* _output_get 30.0)))
  (set `self.Target` (`KismetMathLibrary.SelectFloat` 0.0 (`KismetMathLibrary.SelectFloat` -1.0 1.0 (`|GetInputActionValue`)) (or (and _returnvalue _returnvalue_2) (`KismetMathLibrary.BooleanNOR` _returnvalue _returnvalue_2)))))

(event `self.ReceiveBeginPlay`
  ; EventBegin
  (`|ExecutionSequence`
    (:`then_0`
      (set `self.MaxPlayerHealth` (`/Game/ShootEmUp/Blueprints/AC_Properties.Health` (`self.AC_Properties`)))
      (bind _asbp_game_instance (cast `/Game/ShootEmUp/Core/BP_GameInstance` (`GameplayStatics.GetGameInstance`)))
      (set `self.As BP Game Instance` _asbp_game_instance)
      (`WidgetBlueprintLibrary.SetInputMode_GameOnly` (`GameplayStatics.GetPlayerController` 0)))))

(event `self.ReceiveActorBeginOverlap`
  (params (OtherActor :type "Actor Object Reference"))
  (bind _returnvalue (`self.GetComponentByClass` OtherActor "/Game/ShootEmUp/Blueprints/AC_Properties.AC_Properties_C"))
  (bind _returnvalue_2 (`self.GetComponentByClass` OtherActor "/Game/ShootEmUp/Blueprints/AC_PickUp.AC_PickUp_C"))
  (bind _maxplayerhealth (`self.MaxPlayerHealth`))
  (bind _ac_properties (`self.AC_Properties`))
  (bind _as_bp_game_instance (`self.As BP Game Instance`))
  (bind _firerate (`/Game/ShootEmUp/Blueprints/AC_Properties.Firerate` _ac_properties))
  ; Hit Detection
  (if (`KismetSystemLibrary.IsValid` _returnvalue)
    (if (not (`self.Death`))
      (bind _output_get (set `self.CurrentPlayerHealth` (- (`self.CurrentPlayerHealth`) (`/Game/ShootEmUp/Blueprints/AC_Properties.Damage` _returnvalue))))
      (if (<= _output_get 0.0)
        (`self.PlayerDeath`)
        (else
          (`self.EffectHealth` (/ (`self.CurrentPlayerHealth`) (`self.MaxPlayerHealth`))))))
    (else
      ; Pickup collision
      (if (`KismetSystemLibrary.IsValid` _returnvalue_2)
        (switch `/Game/ShootEmUp/Blueprints/E_PickUpTypes` (`/Game/ShootEmUp/Blueprints/AC_PickUp.PickUpTypes` _returnvalue_2)
          (:`NewEnumerator0`
            ; Health Pickup
            (`self.EffectHealth` (`KismetMathLibrary.FClamp` (+ (`self.CurrentPlayerHealth`) (* _maxplayerhealth 0.2)) 0.0 _maxplayerhealth)))
          (:`NewEnumerator1`
            ; FirerateUp
            (set `/Game/ShootEmUp/Blueprints/AC_Properties.Firerate` (- _firerate (* _firerate 0.1)) _ac_properties))
          (:`NewEnumerator2`
            ; Money
            (bind _output_get_2 (set `self.Money` (`KismetMathLibrary.Conv_Int64ToInt` (`KismetMathLibrary.Round64` (* 1.0 (`self.MoneyMult`))))))
            (if (`KismetSystemLibrary.IsValid` _as_bp_game_instance)
              (`/Game/ShootEmUp/Core/BP_GameInstance.Add Money` _as_bp_game_instance _output_get_2)))
          (:`NewEnumerator3`
            ; Frenzy
            (set `self.FrenzyPowerup` true)
            (`KismetSystemLibrary.Delay` 5.0)
            (set `self.FrenzyPowerup` false)))))))

(event `EffectHealth`
  (params (`Player Health as Percentage` :type "Float (double-precision)"))
  ; HealthBar Event
  (bind _asplayer_controller (cast `PlayerController` (`self.GetController`)))
  (bind _asnew_hud (cast `/Game/ShootEmUp/Core/NewHUD` (`PlayerController.GetHUD` _asplayer_controller)))
  (bind _output_get (set `self.Hud Widget` (`/Game/ShootEmUp/Core/NewHUD.HudWidget` _asnew_hud)))
  (if (`KismetSystemLibrary.IsValid` _output_get)
    (`ProgressBar.SetPercent` (`/Game/ShootEmUp/UI/WBP_PlayerHealth.Health_PB` (`/Game/ShootEmUp/UI/WBP_HUD_Widget.WBP_PlayerHealth` _output_get)) `Player Health as Percentage`)))

(event `InitializeHealth`
  ; Health Reset
  (bind _output_get (set `self.CurrentPlayerHealth` (`self.MaxPlayerHealth`)))
  (`self.EffectHealth` _output_get))

(event `PlayerDeath`
  (bind _returnvalue (`GameplayStatics.GetPlayerController` 0))
  (bind _hud_widget (`self.Hud Widget`))
  ; Death
  (set `self.Death` true)
  (`self.EffectHealth` 0.0)
  (`AudioComponent.Play` (`self.SciFi_Shot_P2__90_`) 0.0)
  (`MeshComponent.SetOverlayMaterial` (`self.StarSparrow01`) "/Game/ShootEmUp/Materials/MI_FlashingEnemyMaterial.MI_FlashingEnemyMaterial")
  (`MovementComponent.StopMovementImmediately` (`self.FloatingPawnMovement`))
  (`self.DisableInput` null)
  (if (`KismetSystemLibrary.IsValid` _hud_widget)
    (bind _returnvalue_2 (`PanelWidget.RemoveChildAt` (`/Game/ShootEmUp/UI/WBP_HUD_Widget.LivesContainer` _hud_widget) 0))
    (if _returnvalue_2
      (`KismetSystemLibrary.Delay` 2.0)
      (`self.SpawnPlayerPawn`)
      (else
        (bind _returnvalue_3 (`|CreateWidget` "/Game/ShootEmUp/UI/WBP_GameOver.WBP_GameOver_C" _returnvalue))
        (`UserWidget.AddToViewport` _returnvalue_3 0)
        (`WidgetBlueprintLibrary.SetInputMode_UIOnlyEx` _returnvalue _returnvalue_3)
        (set `PlayerController.bShowMouseCursor` true _returnvalue)))))

(event `SpawnPlayerPawn`
  ; Respawn
  (set `self.Death` false)
  (bind _returnvalue (`GameplayStatics.GetActorOfClass` "/Script/Engine.PlayerStart"))
  (`self.K2_SetActorLocation` (`self.K2_GetActorLocation` _returnvalue))
  (`self.EnableInput` null)
  (`MeshComponent.SetOverlayMaterial` (`self.StarSparrow01`) null)
  (`self.InitializeHealth`))

(event `InitializeStats`
  (`|ExecutionSequence`))

(fn `UserConstructionScript`)