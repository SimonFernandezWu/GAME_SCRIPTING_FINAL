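; BP_Missile is a shoot-em-up player missile that moves along a scripted path from where it spawns.
; On BeginPlay it stores its start location and plays a timeline whose X and Y tracks set its offset each update.
; X scales by MissileXMult, while Y uses either a fixed negative factor or MissileYMult depending on RightSide, steering the path to a side.
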(event `self.ReceiveBeginPlay`
  (set `self.Initial Location` (`self.K2_GetActorLocation`))
  (bind (_direction _y _x) (`Timeline|Timeline`)
    (:`Update`
      (`self.K2_SetActorLocation` (+ (`KismetMathLibrary.MakeVector` (* _x (`self.MissileXMult`)) (* _y (`KismetMathLibrary.SelectFloat` -400.0 (`self.MissileYMult`) (`self.RightSide`)))) (`self.Initial Location`))))))

(fn `UserConstructionScript`)